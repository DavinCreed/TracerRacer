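; Game mode for a tracer level that randomizes its track layout and ground style on BeginPlay from saved settings.
; It loads MySettingsSave, falling back to a fresh instance, then draws four enabled tracks without repeats.
; Tagged, pre-placed track actors are moved to evenly spaced slots along X rather than spawned.
; It picks a random enabled ground, sinking GroundCity actors for Gridly; City has no handling.
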(event `self.ReceiveBeginPlay`
  (`self.LoadConfig`)
  (`self.GetAvailableTracks`)
  (for (_array_element _array_index) (`self.RandomTracks`)
    (if (>= _array_index 4)
      (break)
      (else
        (`self.MoveTrack` _array_element _array_index))))
  (`self.SelectGroundType`))

(fn `GetAvailableTracks`
  (bind _temptracks (`self.TempTracks`))
  (bind _configinstance (`self.ConfigInstance`))
  (bind _configtracks (`self.ConfigTracks`))
  ;[1 1 1] Get all the selected tracks
  (if (`/Game/Blueprints/MySettingsSave.CfgTrackDebugSetNext` _configinstance)
    (`KismetArrayLibrary.Array_Add` _configtracks "SetNext"))
  (if (`/Game/Blueprints/MySettingsSave.CfgTrackDebugRebuild` _configinstance)
    (`KismetArrayLibrary.Array_Add` _configtracks "Rebuild"))
  (if (`/Game/Blueprints/MySettingsSave.CfgTrackDebugStepInto` _configinstance)
    (`KismetArrayLibrary.Array_Add` _configtracks "StepInto"))
  (if (`/Game/Blueprints/MySettingsSave.CfgTrackDebugBreakAll` _configinstance)
    (`KismetArrayLibrary.Array_Add` _configtracks "BreakAll"))
  (if (`/Game/Blueprints/MySettingsSave.CfgTrackTestingLogFile` _configinstance)
    (`KismetArrayLibrary.Array_Add` _configtracks "LogFile"))
  (if (`/Game/Blueprints/MySettingsSave.CfgTrackTestingBuggy` _configinstance)
    (`KismetArrayLibrary.Array_Add` _configtracks "Buggy"))
  (if (`/Game/Blueprints/MySettingsSave.CfgTrackTestingDefault` _configinstance)
    (`KismetArrayLibrary.Array_Add` _configtracks "Default"))
  (if (`/Game/Blueprints/MySettingsSave.CfgTrackTestingBadData` _configinstance)
    (`KismetArrayLibrary.Array_Add` _configtracks "BadData"))
  ;[1 1 1] Load up the temp track list
  (for _array_element (`self.ConfigTracks`)
    (`KismetArrayLibrary.Array_Add` (`self.TempTracks`) _array_element))
  ;[1 1 1] Randomly sort four of the available tracks
  (for _ (range 4)
    (bind _returnint (`self.GetRandomTrackInt`))
    (`KismetArrayLibrary.Array_Add` (`self.RandomTracks`) (`KismetArrayLibrary.Array_Get` _temptracks _returnint))
    (`KismetArrayLibrary.Array_Remove` _temptracks _returnint)))

(fn `GetRandomTrackInt`
  (returns (ReturnInt :type Integer))
  (return (`KismetMathLibrary.RandomIntegerInRange` 0 (- (`KismetArrayLibrary.Array_Length` (`self.TempTracks`)) 1))))

(fn `LoadConfig`
  (bind _returnvalue (`GameplayStatics.CreateSaveGameObject` "/Game/Blueprints/MySettingsSave.MySettingsSave_C"))
  (bind _asmy_settings_save (cast `/Game/Blueprints/MySettingsSave` _returnvalue))
  (bind _returnvalue_2 (`GameplayStatics.LoadGameFromSlot` (`/Game/Blueprints/MySettingsSave.SaveSlotName` _asmy_settings_save) (`/Game/Blueprints/MySettingsSave.PlayerIndex` _asmy_settings_save)))
  (bind _asmy_settings_save_2 (cast `/Game/Blueprints/MySettingsSave` _returnvalue_2)
    (:`then`
      (set `self.ConfigInstance` _asmy_settings_save_2))
    (:`CastFailed`
      (set `self.ConfigInstance` _asmy_settings_save))))

(fn `MoveTrack`
  (params (TrackName :type String) (Position :type Integer))
  (bind _outactors (`GameplayStatics.GetAllActorsWithTag` (`KismetStringLibrary.Conv_StringToName` TrackName)))
  (for _array_element _outactors
    (`self.K2_SetActorLocation` _array_element (`KismetMathLibrary.MakeVector` (+ (* (`KismetMathLibrary.Conv_IntToDouble` Position) 60000.0) 30000.0)) false false)))

(fn `SelectGroundType`
  (locals (GroundTypes :type "Array of String") (Ground :type String))
  (bind _configinstance (`self.ConfigInstance`))
  (bind _groundtypes (`local.GroundTypes`))
  ;[1 1 1] Load up the available grounds
  (if (`/Game/Blueprints/MySettingsSave.CfgGroundGridly` _configinstance)
    (`KismetArrayLibrary.Array_Add` _groundtypes "Gridly"))
  (if (`/Game/Blueprints/MySettingsSave.CfgGroundCity` _configinstance)
    (`KismetArrayLibrary.Array_Add` _groundtypes "City"))
  ;[1 1 1] Select the random ground
  (bind _output_get (set `local.Ground` (`KismetArrayLibrary.Array_Get` _groundtypes (`KismetMathLibrary.RandomIntegerInRange` 0 (- (`KismetArrayLibrary.Array_Length` _groundtypes) 1)))))
  ;[1 1 1] Setup the grounds
  (switch `string` _output_get
    (:`Gridly`
      (bind _outactors (`GameplayStatics.GetAllActorsWithTag` "GroundCity"))
      (for _array_element _outactors
        (`self.K2_SetActorLocation` _array_element (0.0 0.0 -10000.0) false false)))))

(fn `UserConstructionScript`)
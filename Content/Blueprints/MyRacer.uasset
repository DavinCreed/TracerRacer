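; MyRacer runs a race session for the player character: HUD, pause menu on P, timer and end-of-run saving.
; BeginPlay loads the shop save, or creates one, to set the racer's max speed and health.
; Tick times the run until four gates are passed or hits run out, then calls SaveTheRacer.
; This banks collected Bits and records a time, Bits and health-based high score only for surviving racers.
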(event `self.ReceiveBeginPlay`
  (bind _racer (`self.Racer`))
  (bind _shopinstance (`self.ShopInstance`))
  (bind _health (`/Game/Blueprints/MyShopSave.Health` _shopinstance))
  (bind _returnvalue (`|CreateWidget` "/Game/Blueprints/HUD.HUD_C"))
  (bind _output_get (set `self.HUDReference` _returnvalue))
  (`UserWidget.AddToViewport` _output_get 0)
  (bind _asmy_racer (cast `/Game/Blueprints/MyRacer` (`GameplayStatics.GetPlayerCharacter` 0)))
  (set `self.Racer` _asmy_racer)
  (`WidgetBlueprintLibrary.SetInputMode_GameOnly` (`GameplayStatics.GetPlayerController` 0))
  (bind _returnvalue_2 (`GameplayStatics.CreateSaveGameObject` "/Game/Blueprints/MyShopSave.MyShopSave_C"))
  (bind _asmy_shop_save (cast `/Game/Blueprints/MyShopSave` _returnvalue_2))
  (bind _returnvalue_3 (`GameplayStatics.LoadGameFromSlot` (`/Game/Blueprints/MyShopSave.SaveSlotName` _asmy_shop_save) (`/Game/Blueprints/MyShopSave.PlayerIndex` _asmy_shop_save)))
  (bind _asmy_shop_save_2 (cast `/Game/Blueprints/MyShopSave` _returnvalue_3)
    (:`then`
      (set `self.ShopInstance` _asmy_shop_save_2))
    (:`CastFailed`
      (bind _returnvalue_4 (`GameplayStatics.CreateSaveGameObject` "/Game/Blueprints/MyShopSave.MyShopSave_C"))
      (bind _asmy_shop_save_3 (cast `/Game/Blueprints/MyShopSave` _returnvalue_4))
      (set `self.ShopInstance` _asmy_shop_save_3)))
  (set `RacerClass.SpeedMax` (`/Game/Blueprints/MyShopSave.Speed` _shopinstance) _racer)
  (set `RacerClass.Hits` _health _racer)
  (set `RacerClass.HitsMax` _health _racer)
  (set `self.IsAlive` true))

(event `self.ReceiveTick`
  (params (DeltaSeconds :type "Float (single-precision)"))
  (if (`self.IsAlive`)
    (set `self.TimeCount` (+ DeltaSeconds (`self.TimeCount`)))
    (bind _asmy_racer (cast `/Game/Blueprints/MyRacer` (`self.Racer`)))
    (if (or (>= (`RacerClass.Gates` _asmy_racer) 4) (<= (`RacerClass.Hits` _asmy_racer) 0))
      (`self.SaveTheRacer`))))

(event `Key|P`
  (params (Key :type "Key Structure" :default "AnyKey"))
  (bind _returnvalue (`GameplayStatics.GetPlayerController` 0))
  (bind _pausemenureference (`self.PauseMenuReference`))
  (:`Pressed`
    (bind _asmy_racer (cast `/Game/Blueprints/MyRacer` (`self.Racer`)))
    (if (and (!= (`RacerClass.Gates` _asmy_racer) 4) (!= (`RacerClass.Hits` _asmy_racer) 0))
      (`/Engine/EditorBlueprintResources/StandardMacros.IsValid` (`self.PauseMenuReference`)
        (:`Is Valid`
          _)
        (:`Is Not Valid`
          (bind _returnvalue_2 (`|CreateWidget` "/Game/Blueprints/PauseMenu.PauseMenu_C"))
          (set `self.PauseMenuReference` _returnvalue_2)))
      (`WidgetBlueprintLibrary.SetInputMode_UIOnlyEx` _returnvalue _pausemenureference)
      (`UserWidget.AddToViewport` _pausemenureference 0)
      (`GameplayStatics.SetGamePaused` true)
      (set `PlayerController.bShowMouseCursor` true _returnvalue))))

(event `EndLevel`)

(fn `CurrentHits`
  (returns (ReturnValue :type Integer))
  (return 0))

(fn `GetScore`
  (returns (NewParam :type Integer))
  (bind _racer (`self.Racer`))
  (bind _returnvalue (+ (* (`KismetMathLibrary.Conv_IntToDouble` (`RacerClass.Hits` _racer)) 0.5) 0.5))
  (return (`KismetMathLibrary.Round` (+ (* (* (- 150.0 (`self.TimeCount`)) 1000.0) _returnvalue) (* _returnvalue (* (`KismetMathLibrary.Conv_IntToDouble` (`RacerClass.Bits` _racer)) 100.0))))))

(fn `SaveTheRacer`
  (locals (NewLocalVar_0 :type "/Game/Blueprints/MySaveGame Object Reference"))
  (bind _racer (`self.Racer`))
  (bind _saveinstance (`self.SaveInstance`))
  (bind _bits (`RacerClass.Bits` _racer))
  (if (`self.IsAlive`)
    (set `self.IsAlive` false)
    (bind _returnvalue (`GameplayStatics.CreateSaveGameObject` "/Game/Blueprints/MySaveGame.MySaveGame_C"))
    (bind _asmy_save_game (cast `/Game/Blueprints/MySaveGame` _returnvalue))
    (bind _returnvalue_2 (`GameplayStatics.LoadGameFromSlot` (`/Game/Blueprints/MySaveGame.SaveSlotName` _asmy_save_game) (`/Game/Blueprints/MySaveGame.PlayerIndex` _asmy_save_game)))
    (bind _asmy_save_game_2 (cast `/Game/Blueprints/MySaveGame` _returnvalue_2)
      (:`then`
        (set `self.SaveInstance` _asmy_save_game_2))
      (:`CastFailed`
        (set `self.SaveInstance` _asmy_save_game)))
    (set `/Game/Blueprints/MySaveGame.BitsAmt` (+ (`/Game/Blueprints/MySaveGame.BitsAmt` _saveinstance) _bits) _saveinstance)
    (set `/Game/Blueprints/MySaveGame.BitsTotal` (+ _bits (`/Game/Blueprints/MySaveGame.BitsTotal` _saveinstance)) _saveinstance)
    (bind _newparam (`self.GetScore`))
    (if (and (< (`/Game/Blueprints/MySaveGame.HighScore` _saveinstance) _newparam) (> (`RacerClass.Hits` _racer) 0))
      (set `/Game/Blueprints/MySaveGame.HighScore` _newparam _saveinstance))
    (`GameplayStatics.SaveGameToSlot` _saveinstance (`/Game/Blueprints/MySaveGame.SaveSlotName` _saveinstance) (`/Game/Blueprints/MySaveGame.PlayerIndex` _saveinstance))))

(fn `UserConstructionScript`)
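; Music player actor that plays one random 2D track on BeginPlay, chosen from the songs enabled in the player's settings.
; It loads the MySettingsSave slot, falling back to a newly created save object with default values if loading fails.
; GetRandomSong builds a name list from the music flags and picks one, which a switch maps to a sound cue.
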(event `self.ReceiveBeginPlay`
  (bind _returnvalue (`GameplayStatics.CreateSaveGameObject` "/Game/Blueprints/MySettingsSave.MySettingsSave_C"))
  (bind _asmy_settings_save (cast `/Game/Blueprints/MySettingsSave` _returnvalue))
  (bind _returnvalue_2 (`GameplayStatics.LoadGameFromSlot` (`/Game/Blueprints/MySettingsSave.SaveSlotName` _asmy_settings_save) (`/Game/Blueprints/MySettingsSave.PlayerIndex` _asmy_settings_save)))
  (bind _asmy_settings_save_2 (cast `/Game/Blueprints/MySettingsSave` _returnvalue_2)
    (:`then`
      (set `self.SettingsInstance` _asmy_settings_save_2))
    (:`CastFailed`
      (set `self.SettingsInstance` _asmy_settings_save)))
  (bind _songname (`self.GetRandomSong` (`self.SettingsInstance`)))
  (switch `string` _songname
    (:`NullReference`
      (set `self.CurrentTrack` "/Game/BGM/NullReference_Cue.NullReference_Cue"))
    (:`Debugging`
      (set `self.CurrentTrack` "/Game/BGM/Debugging_Cue.Debugging_Cue"))
    (:`Runtime`
      (set `self.CurrentTrack` "/Game/BGM/Runtime_Cue.Runtime_Cue")))
  (`GameplayStatics.PlaySound2D` (`self.CurrentTrack`)))

(fn `GetRandomSong`
  (params (Config :type "/Game/Blueprints/MySettingsSave Object Reference"))
  (returns (SongName :type String))
  (locals (SongList :type "Array of String"))
  (bind _songlist (`local.SongList`))
  (bind _returnvalue (`KismetArrayLibrary.Array_Length` _songlist))
  (if (`/Game/Blueprints/MySettingsSave.CfgMusicNullReference` Config)
    (`KismetArrayLibrary.Array_Add` _songlist "NullReference"))
  (if (`/Game/Blueprints/MySettingsSave.CfgMusicDebugging` Config)
    (`KismetArrayLibrary.Array_Add` _songlist "Debugging"))
  (if (`/Game/Blueprints/MySettingsSave.CfgMusicRuntime` Config)
    (`KismetArrayLibrary.Array_Add` _songlist "Runtime"))
  (if (== _returnvalue 0)
    (return "")
    (else
      (return (`KismetArrayLibrary.Array_Get` _songlist (`KismetMathLibrary.RandomIntegerInRange` 0 (- _returnvalue 1)))))))

(fn `UserConstructionScript`)